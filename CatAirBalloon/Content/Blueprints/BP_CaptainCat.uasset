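; BP_CaptainCat is an animated cat actor that hops and swivels on its own from BeginPlay.
; Two timelines drive relative Z height and yaw, offset from values cached at start, with X, Y, pitch and roll set to zero.
; Each motion restarts after a random delay while its repeat flag is set, and each swivel gets a random amplitude.
; The cached rotation is a forward vector, whose Z serves as yaw offset.
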(event Custom|Rotate
  (bind _yaw_rotate (Timeline|CatRotate PlayFromStart)
    (:Update
      (Transformation|SetActorRelativeRotation (Math|Rotator|MakeRotator 0.0 0.0 (+ (* _yaw_rotate (Variables|Default|GetRandomRotateScale)) (.z (Variables|Default|GetInitialRotation))))))
    (:Finished
      (if (Variables|Default|GetRepeatRotate)
        (CallFunction|RandomRotate)))))

(event Custom|RandomRotate
  (Utilities|FlowControl|Delay (Math|Random|RandomFloatinRange 0.0 0.5))
  (Variables|Default|SetRandomRotateScale (Math|Random|RandomFloatinRange 1e+01 1e+02))
  (CallFunction|Rotate))

(event Custom|RandomJump
  (Utilities|FlowControl|Delay (Math|Random|RandomFloatinRange 0.0 2.0))
  (CallFunction|Jump))

(event Custom|Jump
  (bind _jump (Timeline|CatJump PlayFromStart)
    (:Update
      (Transformation|SetActorRelativeLocation (Math|Vector|MakeVector 0.0 0.0 (+ (* _jump 1e+02) (.z (Variables|Default|GetInitialLocation))))))
    (:Finished
      (if (Variables|Default|GetRepeatJump)
        (CallFunction|RandomJump)))))

(event EventBeginPlay
  (bind _rootcomponent (Variables|Transformation|GetRootComponent))
  (Variables|Default|SetInitialLocation (Variables|/Script/Engine.SceneComponent|GetRelativeLocation _rootcomponent))
  (Variables|Default|SetInitialRotation (Math|Rotator|GetRotationXVector (Variables|/Script/Engine.SceneComponent|GetRelativeRotation _rootcomponent)))
  (CallFunction|RandomJump)
  (CallFunction|RandomRotate))

(event Collision|EventActorBeginOverlap
  (params (OtherActor :type Actor%20Object%20Reference)))

(event EventTick
  (params (DeltaSeconds :type Float%20%28single-precision%29)))

(fn ConstructionScript)