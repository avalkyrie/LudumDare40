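; Player pawn Blueprint that runs the game's menu flow and plays sound feedback for gameplay events.
; BeginPlay starts theme music and pauses behind a start menu; StartButtonClicked unpauses, swaps in the main HUD and restores game input.
; Event handlers play sounds for air, money, cat and captain events.
; Landing on the ground triggers EndGame, which pauses and replaces the HUD with an end screen.
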(event Custom|EndGame
  (bind _returnvalue (Game|GetPlayerController 0))
  (Game|SetGamePaused true)
  (Widget|RemovefromParent (Variables|Default|GetHUD))
  (bind _returnvalue_2 (UserInterface|CreateWidget "/Game/UI/EndScreen.EndScreen_C"))
  (bind _output_get (Variables|Default|SetEndScreenHUD _returnvalue_2))
  (Variables|/Game/UI/EndScreen.EndScreen_C|SetMyPawn _output_get self)
  (UserInterface|Viewport|AddtoViewport _output_get 0)
  (Input|SetInputModeUIOnly _returnvalue 0 "DoNotLock")
  (Variables|/Script/Engine.PlayerController|SetbShowMouseCursor _returnvalue true))

(event EventBeginPlay
  (bind _returnvalue (Game|GetPlayerController 0))
  (bind _returnvalue_2 (UserInterface|CreateWidget "/Game/UI/StartMenu.StartMenu_C"))
  (bind _output_get (Variables|Default|SetStartMenu _returnvalue_2))
  (UserInterface|Viewport|AddtoViewport _output_get 0) ; Add a start menu to the viewport over the leve, unposses the pawn until "start" button is clicked
  (Variables|/Game/UI/StartMenu.StartMenu_C|SetPlayerPawn _returnvalue_2 self)
  (Game|SetGamePaused true)
  (Input|SetInputModeUIOnly _returnvalue 0 "DoNotLock")
  (Variables|/Script/Engine.PlayerController|SetbShowMouseCursor _returnvalue true)
  (Audio|PlaySound2D "/Game/Assets/Sounds/ThemeSong1.ThemeSong1"))

(event Collision|EventActorBeginOverlap
  (params (OtherActor :type Actor%20Object%20Reference)))

(event EventWarnTerminalVelocity)

(event EventStopWarningTerminalVelocity)

(event EventVentAir
  (Audio|PlaySoundatLocation "/Game/Assets/Sounds/Explosion.Explosion" (Transformation|GetActorLocation)))

(event EventNoAirLeft
  (Audio|PlaySoundatLocation "/Game/Assets/Sounds/Danger.Danger" (Transformation|GetActorLocation)))

(event EventDroppedMoney
  (Audio|PlaySoundatLocation "/Game/Assets/Sounds/DropMoney.DropMoney" (Transformation|GetActorLocation)))

(event EventDroppedCat
  (Audio|PlaySoundatLocation "/Game/Assets/Sounds/EjectCat.EjectCat" (Transformation|GetActorLocation)))

(event EventDidLandonGround
  (Audio|PlaySoundatLocation "/Game/Assets/Sounds/OhNoWarning.OhNoWarning" (Transformation|GetActorLocation))
  (CallFunction|EndGame))

(event EventCaptainJumpedOut
  (Audio|PlaySoundatLocation "/Game/Assets/Sounds/EjectCat.EjectCat" (Transformation|GetActorLocation)))

(event EventTick
  (params (DeltaSeconds :type Float%20%28single-precision%29)))

(event EventPickedUpMoney
  (Audio|PlaySoundatLocation "/Game/Assets/Sounds/CoinGet.CoinGet" (Transformation|GetActorLocation)))

(event EventPickedUpCat
  (Audio|PlaySoundatLocation "/Game/Assets/Sounds/CatGet.CatGet" (Transformation|GetActorLocation)))

(fn ConstructionScript)

(fn StartButtonClicked
  (bind _returnvalue (Game|GetPlayerController 0))
  (Game|SetGamePaused false)
  (bind _returnvalue_2 (UserInterface|CreateWidget "/Game/UI/MainHUD.MainHUD_C"))
  (bind _output_get (Variables|Default|SetHUD _returnvalue_2))
  (Variables|/Game/UI/MainHUD.MainHUD_C|SetMyPawn _output_get self)
  (UserInterface|Viewport|AddtoViewport _output_get 0)
  (Input|SetInputModeGameOnly _returnvalue)
  (Variables|/Script/Engine.PlayerController|SetbShowMouseCursor _returnvalue false)
  (Widget|RemovefromParent (Variables|Default|GetStartMenu)))